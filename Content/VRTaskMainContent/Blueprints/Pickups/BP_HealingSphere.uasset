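; BP_HealingSphere is a VR pickup that restores the local player's health from a limited resource.
; It caches the VR pawn's HealthComponent on BeginPlay, and holding the trigger runs Heal on a looping timer until release.
; Each tick below max health drains Resource and adds HealingAmount, swapping the mesh material once empty.
; The clamped AddedHealth for the last partial charge is computed but not passed to AddHealth.
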(event `self.ReceiveBeginPlay`
  (bind _asbp_vrtpawn (cast `/Game/VRTaskMainContent/Blueprints/Player/BP_VRTPawn` (`Controller.K2_GetPawn` (`VRTaskBlueprintFunctionLibrary.GetLocalPlayerController`))))
  (set `self.PlayerHealthComponent;` (`VRTPawn.HealthComponent` _asbp_vrtpawn)))

(event `VRTInteractableInterface.TriggerPressed`
  (`KismetSystemLibrary.K2_SetTimer` null "Heal" (`self.HealingRate`) true))

(event `VRTInteractableInterface.TriggerReleased`
  (`KismetSystemLibrary.K2_ClearTimer` null "Heal"))

(fn `Heal`
  (locals (AddedHealth :type "Float (double-precision)"))
  (if (> (`self.Resource`) 0.0)
    (bind _playerhealthcomponent_ (`self.PlayerHealthComponent;`)
      (:`then`
        (if (== (`VRTHealthComponent.GetCurrentHealth` _playerhealthcomponent_) (`VRTHealthComponent.MaxHealth` _playerhealthcomponent_))
          (return)
          (else
            (bind _output_get (set `self.Resource` (- (`self.Resource`) (`self.HealingAmount`))))
            (if (== (`KismetMathLibrary.SignOfFloat` _output_get) -1.0)
              (set `local.AddedHealth` (+ (`self.HealingAmount`) (`self.Resource`)))
              (else
                (set `local.AddedHealth` (`self.HealingAmount`))))
            (`VRTHealthComponent.AddHealth` _playerhealthcomponent_ (`self.HealingAmount`))
            (if (<= (`self.Resource`) 0.0)
              (`self.SetEmptySphereMaterial`)))))
      (:`else`))))

(fn `SetEmptySphereMaterial`
  (`PrimitiveComponent.SetMaterial` (`self.StaticMesh`) 0 "/Engine/EngineMaterials/EditorBrushMaterial.EditorBrushMaterial"))

(fn `UserConstructionScript`)